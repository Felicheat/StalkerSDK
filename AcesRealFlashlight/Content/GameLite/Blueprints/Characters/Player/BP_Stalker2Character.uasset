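; Player character Blueprint for Stalker 2 with a flashlight mod, a forward jump boost and a debug key for the XTeleport console command.
; Jumping while moving launches the character forward, with separate forces for walking and other movement.
; Tick scales Perlin-noise spring arm sway by smoothed speed, then polls emission state.
; During emissions, a timeline flickers both spotlights and triggers Wwise flicker sounds; otherwise their base intensities are restored.
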(event `self.OnJumped`
  (bind (_returnvalue_x _returnvalue_y) (`KismetMathLibrary.BreakVector` (* (`SceneComponent.GetForwardVector` (`self.CapsuleComponent`)) 220.0)))
  (bind (_returnvalue_x_2 _returnvalue_y_2) (`KismetMathLibrary.BreakVector` (* (`SceneComponent.GetForwardVector` (`self.CapsuleComponent`)) 125.0)))
  ;[1 0 0.031] JumpForwardForce This need replicate in code
  (if (`CppMediator.IsMoving` self)
    (if (`CppMediator.IsWalking` self)
      (`self.LaunchCharacter` (`KismetMathLibrary.MakeVector` _returnvalue_x _returnvalue_y 1.0))
      (else
        (`self.LaunchCharacter` (`KismetMathLibrary.MakeVector` _returnvalue_x_2 _returnvalue_y_2 1.0))))))

(event `Key|Zero`
  (params (Key :type "Key Structure"))
  ;[1 1 1] Teleporting Menu (GlobalMap)
  (:`Pressed`
    (`KismetSystemLibrary.ExecuteConsoleCommand` "XTeleport" null)))

(event `self.ReceiveBeginPlay`
  ;[1 1 1] Real Flash Light Mod
  (set `self.SpringArm_Loc` (`SceneComponent.RelativeRotation` (`self.SpringArm`)))
  (set `self.FlashlightBase_Int` 21.0)
  (set `self.FakeLightBase_Int` 2.5)
  (`self.CheckEmission` :!label _label))

(event `self.ReceiveTick`
  (params (DeltaSeconds :type "Float (single-precision)"))
  (bind _returnvalue (* (`KismetSystemLibrary.GetGameTimeInSeconds`) (`self.SpringArmWiggle_Speed`)))
  ;[1 1 1] Real Flash Light Mod
  (set `self.SmoothedNormalizedSpeed` (`KismetMathLibrary.FInterpTo` (`self.SmoothedNormalizedSpeed`) (`KismetMathLibrary.FClamp` (`KismetMathLibrary.SafeDivide` (`KismetMathLibrary.VSize` (`self.GetVelocity`)) 760.0) (`self.ClampMin`) (`self.ClampMax`)) DeltaSeconds (`self.SmoothInterpSpeed`)))
  (`SceneComponent.K2_SetRelativeRotation` (`self.SpringArm`) (`KismetMathLibrary.MakeRotator` 0.0 (* (`KismetAnimationLibrary.K2_MakePerlinNoiseAndRemap` (+ _returnvalue 100.0) 0.0 1.0) (* (`self.SpringArmWiggleV_Int`) (`self.SmoothedNormalizedSpeed`))) (* (`KismetAnimationLibrary.K2_MakePerlinNoiseAndRemap` (+ _returnvalue 50.0) -1.0 1.0) (* (`self.SpringArmWiggleH_Int`) (`self.SmoothedNormalizedSpeed`)))) false false)
  (goto _label))

(event `CheckEmission`
  ;[1 1 1] Real Flash Light Mod
  ;;[1 1 1] Emission Flicker WIP
  (bind _returnvalue (`CppMediator.IsEmissionActive`))
  (if _returnvalue
    (`self.FlickOnEmissionStart`)
    (else
      (`self.FlickOffEmissionEnd`))))

(event `FlickOnEmissionStart`
  ;[1 1 1] Real Flash Light Mod
  ;;[1 1 1] Emission Flicker WIP
  (bind (_direction _lightintencitymultiplyer_01) (`Timeline|Timeline_0` :!label _label_2)
    (:`Update`
      (`LightComponent.SetIntensity` (`self.SpotLight`) (* _lightintencitymultiplyer_01 (`self.FlashlightBase_Int`)))
      (`LightComponent.SetIntensity` (`self.SpotLight1`) (* _lightintencitymultiplyer_01 (`self.FakeLightBase_Int`))))
    (:`SoundEvents_01`
      (if (`self.bIsLightOn`)
        (`self.PlayFlickeringSound`)))))

(event `FlickOffEmissionEnd`
  ;[1 1 1] Real Flash Light Mod
  ;;[1 1 1] Emission Flicker WIP
  (`|ExecutionSequence`
    (:`then_0`
      (goto _label_2 :!via `Stop`))
    (:`then_1`
      (`LightComponent.SetIntensity` (`self.SpotLight`) (`self.FlashlightBase_Int`))
      (`LightComponent.SetIntensity` (`self.SpotLight1`) (`self.FakeLightBase_Int`)))))

(fn `PlayFlickeringSound`
  (bind _returnvalue (`AkGameplayStatics.SpawnAkComponentAtLocation` "/Game/_STALKER2/Audio/WwiseAudio/Events/Light_Source/HouseholdLamp/SFX_LightSource_HouseholdLamp_Flicker.SFX_LightSource_HouseholdLamp_Flicker" (`self.K2_GetActorLocation` self) (struct) true))
  (`/Engine/EditorBlueprintResources/StandardMacros.IsValid` _returnvalue
    (:`Is Valid`
      (set `AkComponent.OcclusionRefreshInterval` 0.2 _returnvalue))))

(fn `UserConstructionScript`)