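; BP_Siren_Audio is a one-shot audio actor that plays a Kyiv air-raid siren sound.
; On BeginPlay it waits a short random delay, so multiple sirens can start out of sync, then fades the audio component in.
; The playback-percent event computes the remaining time from the sound's duration and starts a linear fade-out in the final seconds.
; When the audio finishes, the actor destroys itself.
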(event `self.ReceiveBeginPlay`
  (`KismetSystemLibrary.Delay` (`KismetMathLibrary.RandomFloatInRange` 0.0 0.6))
  (`AudioComponent.FadeIn` (`self.kyiv_siren`) 3.0 1.0 0.0 "Linear"))

(event `self.kyiv_siren.OnAudioPlaybackPercent`
  (params (PlayingSoundWave :type "SoundWave Object Reference") (PlaybackPercent :type "Float (single-precision)"))
  (bind _duration (`SoundBase.Duration` (`AudioComponent.Sound` (`self.kyiv_siren`))))
  (if (<= (- _duration (`KismetMathLibrary.Lerp` 0.0 _duration PlaybackPercent)) 3.0)
    (`AudioComponent.FadeOut` (`self.kyiv_siren`) 3.0 0.0 "Linear")))

(event `self.kyiv_siren.OnAudioFinished`
  (`self.K2_DestroyActor`))

(fn `UserConstructionScript`)