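; Example mod for MCM that registers a sample setting of each type, from bool to keybind and button, under "Mod Example 1".
; Interface events register defaults and current values, then copy applied values back into variables.
; AnyKey compares key display names to the keybind to play a sound.
; The button handler checks "Button Test" and "Button Test 2", which don't match the registered "Button Example 1"; BeginPlay adds a debug widget.
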(event `self.ReceiveBeginPlay`
  ;[0.4538 1 0.6823] Debug widget. You may ignore this.
  (bind _returnvalue (`|CreateWidget` "/MCM_ModExample1/MCMExampleDebug.MCMExampleDebug_C" (`GameplayStatics.GetPlayerController` 0)))
  (`UserWidget.AddToViewport` _returnvalue 0))

(event `/ModConfigurationMenu/BPI_MCM_SettingsProvider.RegisterMCMDefaultSettings`
  (params (`BPI MCM API` :type "/ModConfigurationMenu/BPI_MCM_API Interface"))
  (bind _returnvalue (`KismetSystemLibrary.Conv_InterfaceToObject` `BPI MCM API`))
  (message `/ModConfigurationMenu/BPI_MCM_API.RegisterDefaultModSetting` _returnvalue "Mod Example 1" "Float Example 1" "This is a float setting example for MCM." "/MCM_ModExample1/MCM_Header09.MCM_Header09" "Kynes_Peace" "General" "/MCM_ModExample1/MCM_CatHeader12.MCM_CatHeader12" "NewEnumerator2" false 0 (`self.FloatExample1`) 0.1 "" (struct) (0.0 0.0 0.0) (struct) (`|MakeArray` "") 0 "" "")
  (message `/ModConfigurationMenu/BPI_MCM_API.RegisterDefaultModSetting` _returnvalue "Mod Example 1" "Bool Example 1" "This is a bool setting example for MCM." "/MCM_ModExample1/MCM_Header09.MCM_Header09" "Kynes_Peace" "General" "/MCM_ModExample1/MCM_CatHeader12.MCM_CatHeader12" "NewEnumerator0" (`self.BoolExample1`) 0 0.0 0.0 "" (struct) (0.0 0.0 0.0) (struct) (`|MakeArray` "") 0 "" "")
  (message `/ModConfigurationMenu/BPI_MCM_API.RegisterDefaultModSetting` _returnvalue "Mod Example 1" "Int Example 1" "This is an int setting example for MCM." "/MCM_ModExample1/MCM_Header09.MCM_Header09" "Kynes_Peace" "General" "/MCM_ModExample1/MCM_CatHeader12.MCM_CatHeader12" "NewEnumerator1" false (`self.IntExample1`) 0.0 1.0 "" (struct) (0.0 0.0 0.0) (struct) (`|MakeArray` "") 0 "" "")
  (message `/ModConfigurationMenu/BPI_MCM_API.RegisterDefaultModSetting` _returnvalue "Mod Example 1" "String Example 1" "This is a string setting example for MCM." "/MCM_ModExample1/MCM_Header09.MCM_Header09" "Kynes_Peace" "General" "/MCM_ModExample1/MCM_CatHeader12.MCM_CatHeader12" "NewEnumerator3" false 0 0.0 0.0 (`self.StringExample1`) (struct) (0.0 0.0 0.0) (struct) (`|MakeArray` "") 0 "" "")
  (message `/ModConfigurationMenu/BPI_MCM_API.RegisterDefaultModSetting` _returnvalue "Mod Example 1" "Transform Example 1" "This is a transform setting example for MCM." "/MCM_ModExample1/MCM_Header09.MCM_Header09" "Kynes_Peace" "Numbers" "/MCM_ModExample1/MCM_CatHeader04.MCM_CatHeader04" "NewEnumerator4" false 0 0.0 1.0 "" (`self.TransformExample1`) (0.0 0.0 0.0) (struct) (`|MakeArray` "") 0 "" "")
  (message `/ModConfigurationMenu/BPI_MCM_API.RegisterDefaultModSetting` _returnvalue "Mod Example 1" "Vector Example 1" "This is a vector setting example for MCM." "/MCM_ModExample1/MCM_Header09.MCM_Header09" "Kynes_Peace" "Numbers" "/MCM_ModExample1/MCM_CatHeader04.MCM_CatHeader04" "NewEnumerator5" false 0 0.0 0.2 "" (struct) (`self.VectorExample1`) (struct) (`|MakeArray` "") 0 "" "")
  (message `/ModConfigurationMenu/BPI_MCM_API.RegisterDefaultModSetting` _returnvalue "Mod Example 1" "Rotator Example 1" "This is a rotator setting example for MCM." "/MCM_ModExample1/MCM_Header09.MCM_Header09" "Kynes_Peace" "Numbers" "/MCM_ModExample1/MCM_CatHeader04.MCM_CatHeader04" "NewEnumerator6" false 0 0.0 0.01 "" (struct) (0.0 0.0 0.0) (`self.RotatorExample1`) (`|MakeArray` "") 0 "" "")
  (message `/ModConfigurationMenu/BPI_MCM_API.RegisterDefaultModSetting` _returnvalue "Mod Example 1" "Combo Box Example 1" "This is a dropdown or combo box setting example for MCM." "/MCM_ModExample1/MCM_Header09.MCM_Header09" "Kynes_Peace" "General" "/MCM_ModExample1/MCM_CatHeader12.MCM_CatHeader12" "NewEnumerator7" false 0 0.0 0.0 "" (struct) (0.0 0.0 0.0) (struct) (`self.ComboBoxExample`) 0 "" "")
  (message `/ModConfigurationMenu/BPI_MCM_API.RegisterDefaultModSetting` _returnvalue "Mod Example 1" "Custom Keybind Example 1" "This is a custom keybind setting example for MCM." "/MCM_ModExample1/MCM_Header09.MCM_Header09" "Kynes_Peace" "Keybinds" "/MCM_ModExample1/MCM_CatHeader07.MCM_CatHeader07" "NewEnumerator8" false 0 0.0 0.0 "" (struct) (0.0 0.0 0.0) (struct) (`|MakeArray` "") 0 (`self.KeyPressExample1`) "")
  (message `/ModConfigurationMenu/BPI_MCM_API.RegisterDefaultModSetting` _returnvalue "Mod Example 1" "Button Example 1" "This is a button setting example for MCM." "/MCM_ModExample1/MCM_Header09.MCM_Header09" "Kynes_Peace" "Some Button Category" "/MCM_ModExample1/MCM_CatHeader05.MCM_CatHeader05" "NewEnumerator9" false 0 0.0 0.0 "" (struct) (0.0 0.0 0.0) (struct) (`|MakeArray` "") 0 "" "Cool Button"))

(event `/ModConfigurationMenu/BPI_MCM_SettingsProvider.RegisterMCMSettings`
  (params (`BPI MCM API` :type "/ModConfigurationMenu/BPI_MCM_API Interface"))
  (bind _returnvalue (`KismetSystemLibrary.Conv_InterfaceToObject` `BPI MCM API`))
  (`|ExecutionSequence`
    (:`then_0`
      (message `/ModConfigurationMenu/BPI_MCM_API.RegisterModSetting` _returnvalue "Mod Example 1" "Float Example 1" "This is a float setting example for MCM." "/MCM_ModExample1/MCM_Header09.MCM_Header09" "Kynes_Peace" "General" "/MCM_ModExample1/MCM_CatHeader12.MCM_CatHeader12" "NewEnumerator2" false 0 (`self.FloatExample1`) 0.1 "" (struct) (0.0 0.0 0.0) (struct) (`|MakeArray` "") 0 "" "")
      (message `/ModConfigurationMenu/BPI_MCM_API.RegisterModSetting` _returnvalue "Mod Example 1" "Bool Example 1" "This is a bool setting example for MCM." "/MCM_ModExample1/MCM_Header09.MCM_Header09" "Kynes_Peace" "General" "/MCM_ModExample1/MCM_CatHeader12.MCM_CatHeader12" "NewEnumerator0" (`self.BoolExample1`) 0 0.0 0.0 "" (struct) (0.0 0.0 0.0) (struct) (`|MakeArray` "") 0 "" "")
      (message `/ModConfigurationMenu/BPI_MCM_API.RegisterModSetting` _returnvalue "Mod Example 1" "Int Example 1" "This is an int setting example for MCM." "/MCM_ModExample1/MCM_Header09.MCM_Header09" "Kynes_Peace" "General" "/MCM_ModExample1/MCM_CatHeader12.MCM_CatHeader12" "NewEnumerator1" false (`self.IntExample1`) 0.0 1.0 "" (struct) (0.0 0.0 0.0) (struct) (`|MakeArray` "") 0 "" "")
      (message `/ModConfigurationMenu/BPI_MCM_API.RegisterModSetting` _returnvalue "Mod Example 1" "String Example 1" "This is a string setting example for MCM." "/MCM_ModExample1/MCM_Header09.MCM_Header09" "Kynes_Peace" "General" "/MCM_ModExample1/MCM_CatHeader12.MCM_CatHeader12" "NewEnumerator3" false 0 0.0 0.0 (`self.StringExample1`) (struct) (0.0 0.0 0.0) (struct) (`|MakeArray` "") 0 "" "")
      (message `/ModConfigurationMenu/BPI_MCM_API.RegisterModSetting` _returnvalue "Mod Example 1" "Transform Example 1" "This is a transform setting example for MCM." "/MCM_ModExample1/MCM_Header09.MCM_Header09" "Kynes_Peace" "Numbers" "/MCM_ModExample1/MCM_CatHeader04.MCM_CatHeader04" "NewEnumerator4" false 0 0.0 1.0 "" (`self.TransformExample1`) (0.0 0.0 0.0) (struct) (`|MakeArray` "") 0 "" "")
      (message `/ModConfigurationMenu/BPI_MCM_API.RegisterModSetting` _returnvalue "Mod Example 1" "Vector Example 1" "This is a vector setting example for MCM." "/MCM_ModExample1/MCM_Header09.MCM_Header09" "Kynes_Peace" "Numbers" "/MCM_ModExample1/MCM_CatHeader04.MCM_CatHeader04" "NewEnumerator5" false 0 0.0 0.2 "" (struct) (`self.VectorExample1`) (struct) (`|MakeArray` "") 0 "" "")
      (message `/ModConfigurationMenu/BPI_MCM_API.RegisterModSetting` _returnvalue "Mod Example 1" "Rotator Example 1" "This is a rotator setting example for MCM." "/MCM_ModExample1/MCM_Header09.MCM_Header09" "Kynes_Peace" "Numbers" "/MCM_ModExample1/MCM_CatHeader04.MCM_CatHeader04" "NewEnumerator6" false 0 0.0 0.01 "" (struct) (0.0 0.0 0.0) (`self.RotatorExample1`) (`|MakeArray` "") 0 "" "")
      (message `/ModConfigurationMenu/BPI_MCM_API.RegisterModSetting` _returnvalue "Mod Example 1" "Combo Box Example 1" "This is a dropdown or combo box setting example for MCM." "/MCM_ModExample1/MCM_Header09.MCM_Header09" "Kynes_Peace" "General" "/MCM_ModExample1/MCM_CatHeader12.MCM_CatHeader12" "NewEnumerator7" false 0 0.0 0.0 "" (struct) (0.0 0.0 0.0) (struct) (`self.ComboBoxExample`) 0 "" "")
      (message `/ModConfigurationMenu/BPI_MCM_API.RegisterModSetting` _returnvalue "Mod Example 1" "Custom Keybind Example 1" "This is a custom keybind setting example for MCM." "/MCM_ModExample1/MCM_Header09.MCM_Header09" "Kynes_Peace" "Keybinds" "/MCM_ModExample1/MCM_CatHeader07.MCM_CatHeader07" "NewEnumerator8" false 0 0.0 0.0 "" (struct) (0.0 0.0 0.0) (struct) (`|MakeArray` "") 0 (`self.KeyPressExample1`) "")
      (message `/ModConfigurationMenu/BPI_MCM_API.RegisterModSetting` _returnvalue "Mod Example 1" "Button Example 1" "This is a button setting example for MCM." "/MCM_ModExample1/MCM_Header09.MCM_Header09" "Kynes_Peace" "Some Button Category" "/MCM_ModExample1/MCM_CatHeader05.MCM_CatHeader05" "NewEnumerator9" false 0 0.0 0.0 "" (struct) (0.0 0.0 0.0) (struct) (`|MakeArray` "") 0 "" "Cool Button"))
    (:`then_1`
      (message `/ModConfigurationMenu/BPI_MCM_API.AddUniqueModID` _returnvalue "Mod Example 1"))))

(event `/ModConfigurationMenu/BPI_MCM_SettingsProvider.ApplyMCMSettings`
  (params (`BPI MCM API` :type "/ModConfigurationMenu/BPI_MCM_API Interface"))
  (bind _returnvalue (`KismetSystemLibrary.Conv_InterfaceToObject` `BPI MCM API`))
  (bind (_boolvalue _integervalue _floatvalue) (message `/ModConfigurationMenu/BPI_MCM_API.GetModSetting` _returnvalue "Mod Example 1" "Float Example 1"))
  (set `self.FloatExample1` _floatvalue)
  (bind _boolvalue_2 (message `/ModConfigurationMenu/BPI_MCM_API.GetModSetting` _returnvalue "Mod Example 1" "Bool Example 1"))
  (set `self.BoolExample1` _boolvalue_2)
  (bind (_boolvalue_3 _integervalue_2) (message `/ModConfigurationMenu/BPI_MCM_API.GetModSetting` _returnvalue "Mod Example 1" "Int Example 1"))
  (set `self.IntExample1` _integervalue_2)
  (bind (_boolvalue_4 _integervalue_3 _floatvalue_2 _floatcontrollerstepvalue _stringvalue) (message `/ModConfigurationMenu/BPI_MCM_API.GetModSetting` _returnvalue "Mod Example 1" "String Example 1"))
  (set `self.StringExample1` _stringvalue)
  (bind (_boolvalue_5 _integervalue_4 _floatvalue_3 _floatcontrollerstepvalue_2 _stringvalue_2 _transformvalue) (message `/ModConfigurationMenu/BPI_MCM_API.GetModSetting` _returnvalue "Mod Example 1" "Transform Example 1"))
  (set `self.TransformExample1` _transformvalue)
  (bind (_boolvalue_6 _integervalue_5 _floatvalue_4 _floatcontrollerstepvalue_3 _stringvalue_3 _transformvalue_2 _vectorvalue) (message `/ModConfigurationMenu/BPI_MCM_API.GetModSetting` _returnvalue "Mod Example 1" "Vector Example 1"))
  (set `self.VectorExample1` _vectorvalue)
  (bind (_boolvalue_7 _integervalue_6 _floatvalue_5 _floatcontrollerstepvalue_4 _stringvalue_4 _transformvalue_3 _vectorvalue_2 _rotatorvalue) (message `/ModConfigurationMenu/BPI_MCM_API.GetModSetting` _returnvalue "Mod Example 1" "Rotator Example 1"))
  (set `self.RotatorExample1` _rotatorvalue)
  (bind (_boolvalue_8 _integervalue_7 _floatvalue_6 _floatcontrollerstepvalue_5 _stringvalue_5 _transformvalue_4 _vectorvalue_3 _rotatorvalue_2 _comboboxoptions _comboboxselectedoption) (message `/ModConfigurationMenu/BPI_MCM_API.GetModSetting` _returnvalue "Mod Example 1" "Combo Box Example 1"))
  (set `self.ComboBoxChosenString` (`|GetArrayItem` (`self.ComboBoxExample`) _comboboxselectedoption))
  (bind (_boolvalue_9 _integervalue_8 _floatvalue_7 _floatcontrollerstepvalue_6 _stringvalue_6 _transformvalue_5 _vectorvalue_4 _rotatorvalue_3 _comboboxoptions_2 _comboboxselectedoption_2 _type _keybind) (message `/ModConfigurationMenu/BPI_MCM_API.GetModSetting` _returnvalue "Mod Example 1" "Custom Keybind Example 1"))
  (set `self.KeyPressExample1` _keybind))

(event `Key|AnyKey` :consume false :overrideparent false
  (params (Key :type "Key Structure"))
  ;[0.01079 0.0272 0.2188] This is the way I normally create keybinds. So they can be edited in Engine.ini. But in the case of using MCM, you do not need to mark KeyPress variable as Config Variable.
  (:`Pressed`
    (if (`KismetStringLibrary.EqualEqual_StrStr` (`KismetTextLibrary.Conv_TextToString` (`KismetInputLibrary.Key_GetDisplayName` Key false)) (`self.KeyPressExample1`))
      (`GameplayStatics.PlaySound2D` "/Game/_Stalker_2/maps/_Stalker2_WorldMap/QuestObjects/Dialogs/SideQuest/SQ94/SQ94_QC_Zuza_ThirdComplain_VGS.SQ94_QC_Zuza_ThirdComplain_ThirdComplain_80994" 1.0 1.0 0.0 null null))))

(event `/ModConfigurationMenu/BPI_MCM_SettingsProvider.OnMCMButtonPressed`
  (params (ModID :type String) (SettingID :type String))
  ;[1 0.4745 0.4247] This is for buttons, NOT keybinds. Buttons that show up on MCM that do things. For example, when Button Test is pressed, another sound is played. When Button Test 2 is pressed, a console command is executed. You MUST write the button names correctly on the Equal Exactly. So if the button name when registering the button setting is "My Button", here you have to compare the Setting ID to "My Button" instead of "Button Test".
  ;
  ; In this example, we have two buttons registered above called Button Test and Button Test 2. We are comparing when the MCM button is pressed, which one of the two was pressed, and we do whatever we must do according to the one that was pressed.
  (if (and (`KismetStringLibrary.EqualEqual_StrStr` ModID "Mod Example 1") (`KismetStringLibrary.EqualEqual_StrStr` SettingID "Button Test"))
    (`GameplayStatics.PlaySound2D` "/Game/_Stalker_2/maps/_Stalker2_WorldMap/QuestObjects/Dialogs/SideQuest/SQ94/SQ94_QD_Gonta_FirstMeet_VGS.SQ94_QD_Gonta_FirstMeet_Start_not_Legend_73496" 1.0 1.0 0.0 null null)
    (elif (and (`KismetStringLibrary.EqualEqual_StrStr` ModID "Mod Example 1") (`KismetStringLibrary.EqualEqual_StrStr` SettingID "Button Test 2"))
      (`KismetSystemLibrary.ExecuteConsoleCommand` "XCreateItemInInventoryByID Bread 0 10" (`GameplayStatics.GetPlayerController` 0)))))

(fn `UserConstructionScript`)